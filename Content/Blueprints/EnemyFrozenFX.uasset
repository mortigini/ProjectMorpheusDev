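; EnemyFrozenFX is a short-lived effect actor that applies frozen damage to NPCs entering its box.
; On BeginPlay it attaches a particle emitter to its sphere, animates the emitter's scale with a timeline after a delay, then destroys itself.
; Box overlaps cast to NPC and call DamageFrozen with DamageoT, only when the overlapped component's display name contains "Cylinder".
; The delay following that damage call leads to no further action.
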(event `self.ReceiveBeginPlay`
  (bind _sphere (`self.Sphere`))
  (bind _returnvalue (`GameplayStatics.SpawnEmitterAttached` "/Game/SciFiWeapDark/FX/Particles/P_Shotgun_Tracer_Light.P_Shotgun_Tracer_Light" _sphere "None" (0.0 0.0 0.0) (`SceneComponent.K2_GetComponentRotation` _sphere) (`self.EmitterScale`)))
  (set `self.Emitter` _returnvalue)
  (`|ExecutionSequence`
    (:`then_0`
      (`KismetSystemLibrary.Delay` 5.0)
      (`self.K2_DestroyActor`))
    (:`then_1`
      (`KismetSystemLibrary.Delay` 4.0)
      (bind (_direction _scale) (`Timeline|Timeline_0`)
        (:`Update`
          (`SceneComponent.SetWorldScale3D` (`self.Emitter`) (`KismetMathLibrary.Conv_DoubleToVector` _scale)))))))

(event `self.Box.OnComponentBeginOverlap`
  (params (OverlappedComponent :type "PrimitiveComponent Object Reference") (OtherActor :type "Actor Object Reference") (OtherComp :type "PrimitiveComponent Object Reference") (OtherBodyIndex :type Integer) (bFromSweep :type Boolean) (SweepResult :type "HitResult Structure (by ref)"))
  (bind _asnpc (cast `/Game/AI/NPC` OtherActor))
  (if (`KismetStringLibrary.Contains` (`KismetSystemLibrary.GetDisplayName` OtherComp) "Cylinder")
    (`/Game/AI/NPC.DamageFrozen` _asnpc (`self.DamageoT`))
    (`KismetSystemLibrary.Delay` 1.0)))

(fn `UserConstructionScript`)