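; GrenadeEnemy is a timed grenade actor, apparently thrown by enemies, that explodes four seconds after BeginPlay.
; The explosion spawns a particle and sound at the Cube, fires a RadialForce impulse and shakes the player character's camera through RecoilShake.
; It then spawns a PlayerGrenadeExplosionDamageBox, passing Damage and Instigator, and destroys itself.
; Hit events play an attached bounce sound.
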(event `self.ReceiveBeginPlay`
  (bind _returnvalue (`SceneComponent.K2_GetComponentLocation` (`self.Cube`)))
  (`KismetSystemLibrary.Delay` 4.0)
  (`/Engine/EditorBlueprintResources/StandardMacros.DoOnce` false
    (:`Completed`
      (`GameplayStatics.SpawnEmitterAtLocation` "/Game/SciFiWeapDark/FX/Particles/P_Grenade_Explosion_Dark.P_Grenade_Explosion_Dark" _returnvalue (struct) (0.3 0.3 0.3))
      (`GameplayStatics.SpawnSoundAtLocation` "/Game/SciFiWeapDark/Sound/GrenadeLauncher/Wavs/GrenadeLauncher_Explosion01.GrenadeLauncher_Explosion01" _returnvalue (struct) 1.0 1.0 0.0 null null)
      (`|ExecutionSequence`
        (:`then_1`
          (`RadialForceComponent.FireImpulse` (`self.RadialForce`))
          (bind _asthird_person_character (cast `/Game/ThirdPersonBP/Blueprints/ThirdPersonCharacter` (`GameplayStatics.GetPlayerCharacter` 0)))
          (`/Game/ThirdPersonBP/Blueprints/ThirdPersonCharacter.Recoil_Shake` _asthird_person_character 2.0 0.0)
          (`|SpawnActorFromClass` "/Game/Blueprints/PlayerGrenadeExplosionDamageBox.PlayerGrenadeExplosionDamageBox_C" (`KismetMathLibrary.MakeTransform` _returnvalue) "Undefined" "OverrideRootScale" null (`self.Damage`) (`self.Instigator`))
          (`self.K2_DestroyActor`))))))

(event `self.ReceiveHit`
  (params (MyComp :type "PrimitiveComponent Object Reference") (Other :type "Actor Object Reference") (OtherComp :type "PrimitiveComponent Object Reference") (bSelfMoved :type Boolean) (HitLocation :type "Vector Structure") (HitNormal :type "Vector Structure") (NormalImpulse :type "Vector Structure") (Hit :type "HitResult Structure (by ref)"))
  (`GameplayStatics.SpawnSoundAttached` "/Game/SciFiWeapDark/Sound/GrenadeLauncher/GrenadeLauncher_Bounce_Cue.GrenadeLauncher_Bounce_Cue" (`self.Cube`) "None" (0.0 0.0 0.0) (struct) "KeepRelativeOffset" false 1.0 1.0 0.0 null null))

(fn `UserConstructionScript`)