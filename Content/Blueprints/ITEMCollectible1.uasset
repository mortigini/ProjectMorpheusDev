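; Collectible item pickup that adds its ItemInfo to the player's inventory when interacted with.
; BeginPlay picks a default icon from the item type and writes the item name into a world interact widget.
; Nested outer and inner spheres fade the widget text, while another sphere gates interaction, clearing it one second after exit.
; Interact spawns a particle, moves the mesh toward the character's watch socket, notifies the player and destroys the actor.
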(event `self.ReceiveBeginPlay`
  (bind (_item_info_name _item_info_icon _item_info_damagemin _item_info_damagemax _item_info_ammo _item_info_isweapon_ _item_info_isupgrade_ _item_info_isarmor) (break `/Game/Blueprints/ItemInfoStruct` (`self.Item Info`)))
  (bind (_item_info_name_2 _item_info_icon_2 _item_info_damagemin_2 _item_info_damagemax_2 _item_info_ammo_2 _item_info_isweapon__2 _item_info_isupgrade__2 _item_info_isarmor_2 _item_info_isspecial _item_info_damagemultiply_percent _item_info_ammomultiply_percent _item_info_bonushealthfloat _item_info_healthmultiply_percent _item_info_specialweapontype1_2) (break `/Game/Blueprints/ItemInfoStruct` (`self.Item Info`)))
  (bind (_item_info_name_3 _item_info_icon_3 _item_info_damagemin_3 _item_info_damagemax_3 _item_info_ammo_3 _item_info_isweapon__3 _item_info_isupgrade__3 _item_info_isarmor_3 _item_info_isspecial_2 _item_info_damagemultiply_percent_2 _item_info_ammomultiply_percent_2 _item_info_bonushealthfloat_2 _item_info_healthmultiply_percent_2 _item_info_specialweapontype1_2_2) (break `/Game/Blueprints/ItemInfoStruct` (`self.Item Info`)))
  (bind _item_info_name_4 (break `/Game/Blueprints/ItemInfoStruct` (`self.Item Info`)))
  (`|ExecutionSequence`
    (:`then_0`
      (if _item_info_isweapon_
        (set `self.Item Info` (make `/Game/Blueprints/ItemInfoStruct` _item_info_name_2 "/Game/Decals/Pistolet/PistolDecal.PistolDecal" _item_info_damagemin_2 _item_info_damagemax_2 _item_info_ammo_2 _item_info_isweapon__2 _item_info_isupgrade__2 _item_info_isarmor_2 false _item_info_damagemultiply_percent _item_info_ammomultiply_percent _item_info_bonushealthfloat _item_info_healthmultiply_percent _item_info_specialweapontype1_2) :!label _label)
        (elif (and (== _item_info_icon null) _item_info_isarmor)
          (goto _label)
          (elif _item_info_isupgrade_
            (set `self.Item Info` (make `/Game/Blueprints/ItemInfoStruct` _item_info_name_3 "/Game/Decals/Pistolet/3249946.3249946" _item_info_damagemin_3 _item_info_damagemax_3 _item_info_ammo_3 _item_info_isweapon__3 _item_info_isupgrade__3 _item_info_isarmor_3 false _item_info_damagemultiply_percent_2 _item_info_ammomultiply_percent_2 _item_info_bonushealthfloat_2 _item_info_healthmultiply_percent_2 _item_info_specialweapontype1_2_2))))))
    (:`then_1`
      (bind _asinteract_uiwidget_for_items (cast `/Game/UI/InteractUIWidgetForItems` (`WidgetComponent.GetUserWidgetObject` (`self.Widget`))))
      (`TextBlock.SetText` (`/Game/UI/InteractUIWidgetForItems.TextBlock_1` _asinteract_uiwidget_for_items) (`KismetTextLibrary.Conv_StringToText` _item_info_name_4)))))

(event `/Game/Blueprints/Interact.Interact`
  (bind (_item_info_name _item_info_icon) (break `/Game/Blueprints/ItemInfoStruct` (`self.Item Info`)))
  (if (`self.CanInteract?`)
    (`ActorComponent.K2_DestroyComponent` (`self.ww`))
    (set `self.Destroyed` true)
    (`GameplayStatics.SpawnEmitterAtLocation` "/Game/SciFiWeapDark/FX/Particles/IntelCollectibleParticle.IntelCollectibleParticle" (`SceneComponent.K2_GetComponentLocation` (`self.Intel`)) (struct) (0.7 0.7 0.7))
    (bind _asthird_person_character (cast `/Game/ThirdPersonBP/Blueprints/ThirdPersonCharacter` (`GameplayStatics.GetPlayerCharacter` 0)))
    (`KismetSystemLibrary.MoveComponentTo` (`self.Intel`) (`SceneComponent.GetSocketLocation` (`Character.Mesh` _asthird_person_character) "WatchSocket") (struct) true true 0.3)
    (bind _asthird_person_character_2 (cast `/Game/ThirdPersonBP/Blueprints/ThirdPersonCharacter` (`GameplayStatics.GetPlayerCharacter` 0)))
    (`/Game/UI/InventoryScreen.AddToInventory` (`/Game/ThirdPersonBP/Blueprints/ThirdPersonCharacter.Inventory` _asthird_person_character_2) (`self.Item Info`))
    (`/Game/ThirdPersonBP/Blueprints/ThirdPersonCharacter.NewItemAdded` _asthird_person_character_2 (`KismetTextLibrary.Conv_StringToText` _item_info_name) _item_info_icon)
    (`self.K2_DestroyActor`)))

(event `self.Sphere.OnComponentBeginOverlap`
  (params (OverlappedComponent :type "PrimitiveComponent Object Reference") (OtherActor :type "Actor Object Reference") (OtherComp :type "PrimitiveComponent Object Reference") (OtherBodyIndex :type Integer) (bFromSweep :type Boolean) (SweepResult :type "HitResult Structure (by ref)"))
  (if (== (`KismetSystemLibrary.GetDisplayName` OtherActor) "ThirdPersonCharacter")
    (set `self.CanInteract?` true)))

(event `self.Sphere.OnComponentEndOverlap`
  (params (OverlappedComponent :type "PrimitiveComponent Object Reference") (OtherActor :type "Actor Object Reference") (OtherComp :type "PrimitiveComponent Object Reference") (OtherBodyIndex :type Integer))
  (if (== (`KismetSystemLibrary.GetDisplayName` OtherActor) "ThirdPersonCharacter")
    (`KismetSystemLibrary.Delay` 1.0)
    (set `self.CanInteract?` false)))

(event `self.ReceiveTick`
  (params (DeltaSeconds :type "Float (single-precision)"))
  (if (not (`self.Destroyed`))
    (`SceneComponent.K2_SetWorldRotation` :`self` (`self.ww`))))

(event `self.OutherSphere.OnComponentBeginOverlap`
  (params (OverlappedComponent :type "PrimitiveComponent Object Reference") (OtherActor :type "Actor Object Reference") (OtherComp :type "PrimitiveComponent Object Reference") (OtherBodyIndex :type Integer) (bFromSweep :type Boolean) (SweepResult :type "HitResult Structure (by ref)"))
  (cast `/Game/ThirdPersonBP/Blueprints/ThirdPersonCharacter` OtherActor)
  (bind _asinteract_uiwidget_for_items (cast `/Game/UI/InteractUIWidgetForItems` (`WidgetComponent.GetUserWidgetObject` (`self.Widget`))))
  (`/Game/UI/InteractUIWidgetForItems.FadeInTextLowerr` _asinteract_uiwidget_for_items))

(event `self.OutherSphere.OnComponentEndOverlap`
  (params (OverlappedComponent :type "PrimitiveComponent Object Reference") (OtherActor :type "Actor Object Reference") (OtherComp :type "PrimitiveComponent Object Reference") (OtherBodyIndex :type Integer))
  (cast `/Game/ThirdPersonBP/Blueprints/ThirdPersonCharacter` OtherActor)
  (bind _asinteract_uiwidget_for_items (cast `/Game/UI/InteractUIWidgetForItems` (`WidgetComponent.GetUserWidgetObject` (`self.Widget`))))
  (`/Game/UI/InteractUIWidgetForItems.FadeOutTextLowerr` _asinteract_uiwidget_for_items))

(event `self.InnerSphere.OnComponentBeginOverlap`
  (params (OverlappedComponent :type "PrimitiveComponent Object Reference") (OtherActor :type "Actor Object Reference") (OtherComp :type "PrimitiveComponent Object Reference") (OtherBodyIndex :type Integer) (bFromSweep :type Boolean) (SweepResult :type "HitResult Structure (by ref)"))
  (cast `/Game/ThirdPersonBP/Blueprints/ThirdPersonCharacter` OtherActor)
  (bind _asinteract_uiwidget_for_items (cast `/Game/UI/InteractUIWidgetForItems` (`WidgetComponent.GetUserWidgetObject` (`self.Widget`))))
  (`/Game/UI/InteractUIWidgetForItems.FadeInTexxt` _asinteract_uiwidget_for_items))

(event `self.InnerSphere.OnComponentEndOverlap`
  (params (OverlappedComponent :type "PrimitiveComponent Object Reference") (OtherActor :type "Actor Object Reference") (OtherComp :type "PrimitiveComponent Object Reference") (OtherBodyIndex :type Integer))
  (cast `/Game/ThirdPersonBP/Blueprints/ThirdPersonCharacter` OtherActor)
  (bind _asinteract_uiwidget_for_items (cast `/Game/UI/InteractUIWidgetForItems` (`WidgetComponent.GetUserWidgetObject` (`self.Widget`))))
  (`/Game/UI/InteractUIWidgetForItems.FadeOutTexxt` _asinteract_uiwidget_for_items))

(fn `UserConstructionScript`)