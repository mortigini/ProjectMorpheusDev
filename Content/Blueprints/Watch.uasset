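; Watch actor that gives the player pickup feedback on its Face component for new items, intel and EXP.
; Intel and EXP events swap the Face material, then restore the default after a one-second retriggerable delay.
; Item and intel events play the same attached pickup sound, while EXP is silent.
; The new item event only resets the material after its delay, without setting a highlight.
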(event `self.ReceiveBeginPlay`)

(event `NewItemAdded`
  (`GameplayStatics.SpawnSoundAttached` "/Game/SciFiWeapDark/Sound/GrenadeLauncher/GrenadeLauncher_AmmoPickup_Cue.GrenadeLauncher_AmmoPickup_Cue" (`self.Face`) "None" (0.0 0.0 0.0) (struct) "KeepRelativeOffset" false 1.0 1.0 0.0 null null)
  (`KismetSystemLibrary.RetriggerableDelay` 1.0)
  (`PrimitiveComponent.SetMaterial` (`self.Face`) 0 (`self.DefaultMaterial`)))

(event `IntelAdded`
  (`GameplayStatics.SpawnSoundAttached` "/Game/SciFiWeapDark/Sound/GrenadeLauncher/GrenadeLauncher_AmmoPickup_Cue.GrenadeLauncher_AmmoPickup_Cue" (`self.Face`) "None" (0.0 0.0 0.0) (struct) "KeepRelativeOffset" false 1.0 1.0 0.0 null null)
  (`PrimitiveComponent.SetMaterial` (`self.Face`) 0 "/Game/IntelCollectible.IntelCollectible")
  (`KismetSystemLibrary.RetriggerableDelay` 1.0)
  (`PrimitiveComponent.SetMaterial` (`self.Face`) 0 (`self.DefaultMaterial`)))

(event `EXPAdded`
  (`PrimitiveComponent.SetMaterial` (`self.Face`) 0 "/Game/HealthHalfMatIns1.HealthHalfMatIns1")
  (`KismetSystemLibrary.RetriggerableDelay` 1.0)
  (`PrimitiveComponent.SetMaterial` (`self.Face`) 0 (`self.DefaultMaterial`)))

(fn `UserConstructionScript`)